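; BP_PowerPanel is an interactable power panel that counts toward activating all switchboards in LeaveMeAlone.
; Its Interact event runs once, turns the ActivationLight green and sets IsActivated to false, unless the light is already green.
; It then increments ActivatedPanels on GM_LeaveMeAlone, capped at three, and sets AllPanelsActivated there when that count is reached.
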(event `InteractableInterface.Interact`
  (params (Instigator :type "Actor Object Reference"))
  (`/Engine/EditorBlueprintResources/StandardMacros.DoOnce` false
    (:`Completed`
      (if (!= (`LightComponentBase.GetLightColor` (`self.ActivationLight`)) (struct :`R` 0.05 :`G` 1.0 :`B` 0.05 :`A` 1.0))
        (set `self.bIsActivated` false)
        (`LightComponent.SetLightColor` (`self.ActivationLight`) (struct :`R` 0.05 :`G` 1.0 :`B` 0.05 :`A` 1.0) true)
        (bind _asgm_leave_me_alone (cast `/Game/LeaveMeAlone/Core/GameMode/GM_LeaveMeAlone` (`GameplayStatics.GetGameMode`)))
        (bind _output_get (set `/Game/LeaveMeAlone/Core/GameMode/GM_LeaveMeAlone.ActivatedPanels` (`KismetMathLibrary.Min` (+ (`/Game/LeaveMeAlone/Core/GameMode/GM_LeaveMeAlone.ActivatedPanels` _asgm_leave_me_alone) 1) 3) _asgm_leave_me_alone))
        (if (>= _output_get 3)
          (set `/Game/LeaveMeAlone/Core/GameMode/GM_LeaveMeAlone.bAllPanelsActivated` true _asgm_leave_me_alone))))))

(fn `UserConstructionScript`)
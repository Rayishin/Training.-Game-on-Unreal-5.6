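; BP_KeyCard is a key card pickup that registers itself with the game mode when collected.
; A short delay after BeginPlay enables collection through the Sphere's begin-overlap event.
; That event casts player character 0 to LMADefaultCharacter without checking the overlapping actor, then calls AddKeyCard on GM_LeaveMeAlone and destroys the card.
; The IsCollected guard is only ever set to false, so it never blocks a pickup.
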(event `self.ReceiveBeginPlay`
  (`KismetSystemLibrary.Delay` 0.5)
  (set `self.bCanCollect` true))

(event `self.Sphere.OnComponentBeginOverlap`
  (params (OverlappedComponent :type "PrimitiveComponent Object Reference") (OtherActor :type "Actor Object Reference") (OtherComp :type "PrimitiveComponent Object Reference") (OtherBodyIndex :type Integer) (bFromSweep :type Boolean) (SweepResult :type "HitResult Structure (by ref)"))
  (if (`self.bCanCollect`)
    (cast `LMADefaultCharacter` (`GameplayStatics.GetPlayerCharacter` 0))
    (if (not (`self.IsCollected`))
      (set `self.IsCollected` false)
      (bind _asgm_leave_me_alone (cast `/Game/LeaveMeAlone/Core/GameMode/GM_LeaveMeAlone` (`GameplayStatics.GetGameMode`)))
      (`/Game/LeaveMeAlone/Core/GameMode/GM_LeaveMeAlone.AddKeyCard` _asgm_leave_me_alone)
      (`self.K2_DestroyActor`))))

(fn `UserConstructionScript`)
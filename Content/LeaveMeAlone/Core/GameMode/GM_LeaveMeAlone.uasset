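; GM_LeaveMeAlone is the game mode that runs the match countdown and ends the game when time runs out.
; On BeginPlay a looping one-second timer decrements GameTime.
; At zero it shows the WBP_TimesUp widget with the CH_Player's Score, switches input to UI only, pauses the game and clears the timer.
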(event `self.ReceiveBeginPlay`
  (bind _returnvalue (`KismetSystemLibrary.K2_SetTimerDelegate` (delegate `CustomEvent`) 1.0 true))
  (set `self.Game Timer Handle` _returnvalue))

(event `CustomEvent`
  (bind _output_get (set `self.Game Time` (- (`self.Game Time`) 1)))
  (if (== _output_get 0)
    (bind _asch_player (cast `/Game/LeaveMeAlone/Core/Characters/CH_Player` (`GameplayStatics.GetPlayerCharacter` 0)))
    (bind _returnvalue (`|CreateWidget` "/Game/LeaveMeAlone/Widgets/UI/WBP_TimesUp.WBP_TimesUp_C" null (`/Game/LeaveMeAlone/Core/Characters/CH_Player.Score` _asch_player)))
    (`UserWidget.AddToViewport` _returnvalue 0)
    (`WidgetBlueprintLibrary.SetInputMode_UIOnlyEx` (`GameplayStatics.GetPlayerController` 0) _returnvalue)
    (`GameplayStatics.SetGamePaused` true)
    (`KismetSystemLibrary.K2_ClearAndInvalidateTimerHandle` (`self.Game Timer Handle`))))

(fn `UserConstructionScript`)